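; Player character pawn with camera-relative movement, look input, sprinting, a coin counter, ladder climbing and scroll-based goal and death states.
; Settrue and Setfalse toggle ladder flying mode, where E plays a timeline that drives upward movement input.
; Scroll pickup disables movement and prints a goal message; first damage disables movement, sets a short lifespan and the Ragdoll profile without simulating physics.
; C adds debug coins, and a looping sprint-risk timer is a stub without coin dropping.
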(event Custom|ObtaionScroll
  (Pawn|Components|CharacterMovement|DisableMovement (Variables|Character|GetCharacterMovement))
  (Variables|Default|SetHasCroll true)
  (Utilities|FlowControl|Delay 3.0)
  (Development|PrintString "Goal!"))

(event EventBeginPlay
  (Variables|/Script/Engine.CharacterMovementComponent|SetMaxWalkSpeed (Variables|Character|GetCharacterMovement) (Variables|Pawn|Character|GetGroundWalkSpeed))
  (Utilities|Time|SetTimerbyFunctionName 0 "CheckSprintRisk" 0.5 true))

(event Collision|EventActorBeginOverlap
  (params (OtherActor :type Actor%20Object%20Reference)))

(event EventTick
  (params (DeltaSeconds :type Float%20%28single-precision%29)))

(event Game|Damage|EventAnyDamage
  (params (Damage :type Float%20%28single-precision%29) (DamageType :type Damage%20Type%20Object%20Reference) (InstigatedBy :type Controller%20Object%20Reference) (DamageCauser :type Actor%20Object%20Reference))
  (bind _mesh (Variables|Character|GetMesh))
  (Utilities|FlowControl|DoOnce false
    (:Completed
      (Development|PrintString "Died!")
      (Pawn|Components|CharacterMovement|DisableMovement (Variables|Character|GetCharacterMovement))
      (Actor|SetLifeSpan 3.0)
      (Collision|SetCollisionProfileName _mesh "Ragdoll" :!class /Script/Engine.PrimitiveComponent)
      (Physics|SetSimulatePhysics _mesh false))))

(event Input|ActionEvents|InputActionSprint
  (params (Key :type Key%20Structure :default "None"))
  (bind _charactermovement (Variables|Character|GetCharacterMovement))
  (:Pressed
    (Variables|/Script/Engine.CharacterMovementComponent|SetMaxWalkSpeed _charactermovement (Variables|Pawn|Character|GetGroundSprintSpeed)))
  (:Released
    (Variables|/Script/Engine.CharacterMovementComponent|SetMaxWalkSpeed _charactermovement (Variables|Pawn|Character|GetGroundWalkSpeed))))

(event Input|AxisEvents|InputAxisMoveForward
  (params (AxisValue :type Float%20%28single-precision%29))
  (Pawn|Input|AddMovementInput (CallFunction|FlattenDirection (Math|Vector|GetForwardVector (Variables|Default|GetCamera))) AxisValue false))

(event Input|AxisEvents|InputAxisMoveRight
  (params (AxisValue :type Float%20%28single-precision%29))
  (Pawn|Input|AddMovementInput (CallFunction|FlattenDirection (Math|Vector|GetRightVector (Variables|Default|GetCamera))) AxisValue false))

(event Input|AxisEvents|InputAxisLookUp
  (params (AxisValue :type Float%20%28single-precision%29))
  (Pawn|Input|AddControllerPitchInput AxisValue))

(event Input|AxisEvents|InputAxisLookRight
  (params (AxisValue :type Float%20%28single-precision%29))
  (Pawn|Input|AddControllerYawInput AxisValue))

(event Input|KeyboardEvents|C
  (params (Key :type Key%20Structure :default "None"))
  (:Pressed
    (bind _aspnplayer_pawn (Utilities|Casting|CastToPNPlayerPawn (Game|Player|GetPlayerPawn 0)))
    (CallFunction|AddCoin _aspnplayer_pawn 5)))

(event Input|KeyboardEvents|E
  (params (Key :type Key%20Structure :default "None"))
  (:Pressed
    (if (Variables|Default|GetLadder)
      (bind _새_트랙_0 (Timeline|타임라인_0 PlayFromStart)
        (:Update
          (Pawn|Input|AddMovementInput (* "0,0.000000,100.000000" _새_트랙_0) 1.0 false))))))

(fn ConstructionScript)

(fn AddCoin
  (params (Num :type Integer))
  (bind _output_get (Variables|Default|SetNumOfCoins (+ (Variables|Default|GetNumOfCoins) Num)))
  (Development|PrintString (Utilities|String|ToString(Integer) _output_get)))

(fn GetNumofCoins
  (return (Variables|Default|GetNumOfCoins)))

(fn CheckSprintRisk
  (if (>= (Utilities|GetFlatSpeed) (Variables|Pawn|Character|GetGroundSprintSpeed))
    (Development|PrintString "") ; DropCoin 함수 호출해야 되지만 나는 안함~
  ))

(fn Settrue
  (Variables|Default|SetLadder true)
  (Pawn|Components|CharacterMovement|SetMovementMode (Variables|Character|GetCharacterMovement) "MOVE_Flying" 0))

(fn Setfalse
  (Variables|Default|SetLadder false)
  (Pawn|Components|CharacterMovement|SetMovementMode (Variables|Character|GetCharacterMovement) "MOVE_Walking" 0))