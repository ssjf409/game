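; PN_Ladder is a climbable ladder actor that tells the player pawn when climbing is possible.
; When a PNPlayerPawn begins overlapping CollisionComponent below its center, it prints an "E" climb prompt and sets a boolean on the pawn.
; Ending the overlap prints a step-up message and clears that boolean.
; The actor itself handles neither input nor climbing movement.
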(event OnComponentBeginOverlap(CollisionComponent)
  (params (OverlappedComponent :type Primitive%20Component%20Object%20Reference) (OtherActor :type Actor%20Object%20Reference) (OtherComp :type Primitive%20Component%20Object%20Reference) (OtherBodyIndex :type Integer) (bFromSweep :type Boolean) (SweepResult :type Hit%20Result%20Structure%20%28by%20ref%29))
  (bind _aspnplayer_pawn (Utilities|Casting|CastToPNPlayerPawn OtherActor))
  (if (> (.Z (Math|Vector|BreakVector (Transformation|GetWorldLocation (Variables|Default|GetCollisionComponent)))) (.Z (Math|Vector|BreakVector (Transformation|GetActorLocation _aspnplayer_pawn))))
    (Development|PrintString "E : 벽타기!")
    (Default|Settrue _aspnplayer_pawn)))

(event OnComponentEndOverlap(CollisionComponent)
  (params (OverlappedComponent :type Primitive%20Component%20Object%20Reference) (OtherActor :type Actor%20Object%20Reference) (OtherComp :type Primitive%20Component%20Object%20Reference) (OtherBodyIndex :type Integer))
  (bind _aspnplayer_pawn (Utilities|Casting|CastToPNPlayerPawn OtherActor))
  (Development|PrintString "발돋음하세요!")
  (Default|Setfalse _aspnplayer_pawn))

(event EventBeginPlay)

(event Collision|EventActorBeginOverlap
  (params (OtherActor :type Actor%20Object%20Reference)))

(event EventTick
  (params (DeltaSeconds :type Float%20%28single-precision%29)))

(fn ConstructionScript)